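; FoodBP is a food actor that counts overlaps as food eaten and triggers the win screen.
; On BeginPlay it sweeps its Sphere component to a fixed world position.
; Each actor overlap increments FoodEated, with no filter on the overlapping actor and no move or destroy afterward.
; When the count equals 95, it adds the W_Win widget to the viewport and pauses the game.
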(event EventBeginPlay
  (Transformation|SetWorldLocation (Variables|Default|GetSphere) "-250.000000,-250.000000,55.000000" true false))

(event Collision|EventActorBeginOverlap
  (params (OtherActor :type Actor%20Object%20Reference))
  (bind _result (Math|Integer|IncrementInt (Variables|Default|GetFoodEated))
    (:%20%20
      (bind _output_get (Variables|Default|SetFoodEated _result))
      (if (== _output_get 95)
        (bind _returnvalue (UserInterface|CreateWidget "/Game/W_Win.W_Win_C" (Game|GetPlayerController 0)))
        (UserInterface|Viewport|AddtoViewport _returnvalue 0)
        (Game|SetGamePaused true)))))

(event EventTick
  (params (DeltaSeconds :type Float%20%28single-precision%29)))

(fn ConstructionScript)