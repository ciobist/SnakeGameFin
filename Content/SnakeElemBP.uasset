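; Snake body segment Blueprint that handles game over on collision and gives the first segment its own material.
; BeginPlay moves each segment to a fixed start location.
; On overlap, if the first SnakeElemBP found also overlaps that actor, it raises the saved high score to FoodBP's eaten count if higher, saves, then reopens Main after a delay.
; SetFirstElementType extends the parent call with the material swap.
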(event EventBeginPlay
  (Transformation|SetActorLocation "450.000000,50.000000,55.000000" false false))

(event Collision|EventActorBeginOverlap
  (params (OtherActor :type Actor%20Object%20Reference))
  (bind _outactors (Actor|GetAllActorsOfClass "SnakeElemBP_C"))
  (if (Collision|IsOverlappingActor (Utilities|Array|Get(acopy) _outactors) OtherActor :!class /Script/Engine.Actor)
    (bind _outactors_2 (Actor|GetAllActorsOfClass "/Game/FoodBP.FoodBP_C"))
    (bind _asfood_bp (Utilities|Casting|CastToFoodBP (Utilities|Array|Get(acopy) _outactors_2)))
    (bind _returnvalue (SaveGame|LoadGamefromSlot "HIghScore"))
    (bind _assave_game (Utilities|Casting|CastToSave_Game _returnvalue))
    (if (> (Variables|/Game/Save_Game.Save_Game_C|GetHighScore _assave_game) (Variables|/Game/FoodBP.FoodBP_C|GetFoodEated _asfood_bp))
      _
      (else
        (Variables|/Game/Save_Game.Save_Game_C|SetHighScore _assave_game (Variables|/Game/FoodBP.FoodBP_C|GetFoodEated _asfood_bp))
        (Utilities|FlowControl|Delay 0.2)))
    (SaveGame|SaveGametoSlot _assave_game "HighScore")
    (Utilities|FlowControl|Delay 1.8)
    (Game|OpenLevel(byName) "Main")))

(event EventTick
  (params (DeltaSeconds :type Float%20%28single-precision%29)))

(event EventSetFirstElementType
  (|CallParentFunction)
  (Rendering|Material|SetMaterial (Variables|Default|GetMeshComponent) 0 "/Engine/MapTemplates/Materials/BasicAsset03.BasicAsset03"))

(fn ConstructionScript)